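; Tutorial light actor whose point light the player adjusts from inside a trigger, which enables input and toggles help and intensity text.
; Keys raise or lower intensity, flip between bright and dim, or randomize color, with intensity changes refreshing the readout.
; Tick runs a looped countdown of a separate intensity variable into the light, then blinks it using delays drawn from random factors of ten.
; GetNumberInRange is defined but never called.
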(event OnComponentBeginOverlap(Trigger)
  (params (OverlappedComponent :type Primitive%20Component%20Object%20Reference) (OtherActor :type Actor%20Object%20Reference) (OtherComp :type Primitive%20Component%20Object%20Reference) (OtherBodyIndex :type Integer) (bFromSweep :type Boolean) (SweepResult :type Hit%20Result%20Structure%20%28by%20ref%29))
  (Input|EnableInput (Game|GetPlayerController 0))
  (Rendering|ToggleVisibility (Variables|Default|GetHelpfulText) false)
  (Rendering|Components|TextRender|SetText (Variables|Default|GetInsensityVolume) (Utilities|Text|ToText(Float) (Variables|/Script/Engine.LightComponentBase|GetIntensity (Variables|Default|GetPointLight)) "HalfToEven")) ; Show Intensity Volume
)

(event OnComponentEndOverlap(Trigger)
  (params (OverlappedComponent :type Primitive%20Component%20Object%20Reference) (OtherActor :type Actor%20Object%20Reference) (OtherComp :type Primitive%20Component%20Object%20Reference) (OtherBodyIndex :type Integer))
  (Input|DisableInput (Game|GetPlayerController 0))
  (Rendering|ToggleVisibility (Variables|Default|GetHelpfulText) false)
  (Rendering|Components|TextRender|SetText (Variables|Default|GetInsensityVolume) (Utilities|Text|ToText(Float) (Variables|/Script/Engine.LightComponentBase|GetIntensity (Variables|Default|GetPointLight)) "HalfToEven")) ; Show Intensity Volume
)

(event EventBeginPlay
  (Rendering|SetVisibility (Variables|Default|GetPointLight) (Variables|Default|Getintensity) false))

(event EventTick
  (params (DeltaSeconds :type Float%20%28single-precision%29))
  (bind _pointlight (Variables|Default|GetPointLight))
  (Utilities|FlowControl|Sequence
    (:then_0
      (if (> (Variables|Default|GetLightIntensity) 1.0) :!label _label
        (Utilities|FlowControl|FlipFlop
          (:A
            _)
          (:B
            _))
        (bind _output_get (Variables|Default|SetLightIntensity (- (Variables|Default|GetLightIntensity) 1.0)))
        (Rendering|Components|Light|SetIntensity (Variables|Default|GetPointLight) _output_get)
        (goto _label)
        (else
          (Development|PrintString "Insensity 1" false false "(R=0.000000,G=0.660000,B=1.000000,A=1.000000)" 0.2))))
    (:then_1
      (Rendering|SetVisibility _pointlight true false)
      (Utilities|FlowControl|Delay (Math|Conversions|ToFloat(Integer) (stale _num)))
      (bind _num (CallFunction|GetNumFactorOf 10))
      (Rendering|SetVisibility _pointlight false false))))

(event Input|KeyboardEvents|P
  (params (Key :type Key%20Structure))
  (bind _pointlight (Variables|Default|GetPointLight))
  (:Pressed
    (Utilities|FlowControl|FlipFlop
      (:A
        (Rendering|Components|Light|SetIntensity _pointlight 5e+04))
      (:B
        (Rendering|Components|Light|SetIntensity _pointlight 1.0)))
    (Rendering|Components|TextRender|SetText (Variables|Default|GetInsensityVolume) (Utilities|Text|ToText(Float) (Variables|/Script/Engine.LightComponentBase|GetIntensity (Variables|Default|GetPointLight)) "HalfToEven")) ; Show Intensity Volume
  ))

(event Input|KeyboardEvents|O
  (params (Key :type Key%20Structure))
  (:Pressed
    (bind _output_get (Variables|Default|SetLight%20Color (Utilities|Struct|MakeLinearColor (Math|Random|RandomFloat) (Math|Random|RandomFloat) (Math|Random|RandomFloat) 1.0)))
    (Rendering|Components|Light|SetLightColor (Variables|Default|GetPointLight) _output_get true)
    (Utilities|FlowControl|Sequence)))

(event Input|KeyboardEvents|I
  (params (Key :type Key%20Structure))
  (bind _pointlight (Variables|Default|GetPointLight))
  (:Pressed
    (Rendering|Components|Light|SetIntensity _pointlight (+ (Variables|/Script/Engine.LightComponentBase|GetIntensity _pointlight) 1e+03))
    (Rendering|Components|TextRender|SetText (Variables|Default|GetInsensityVolume) (Utilities|Text|ToText(Float) (Variables|/Script/Engine.LightComponentBase|GetIntensity _pointlight) "HalfToEven")) ; Show Intensity Volume
  ))

(event Input|KeyboardEvents|K
  (params (Key :type Key%20Structure))
  (bind _pointlight (Variables|Default|GetPointLight))
  (:Pressed
    (Rendering|Components|Light|SetIntensity _pointlight (- (Variables|/Script/Engine.LightComponentBase|GetIntensity _pointlight) 1e+03))
    (Rendering|Components|TextRender|SetText (Variables|Default|GetInsensityVolume) (Utilities|Text|ToText(Float) (Variables|/Script/Engine.LightComponentBase|GetIntensity (Variables|Default|GetPointLight)) "HalfToEven")) ; Show Intensity Volume
  ))

(fn ConstructionScript)

(fn GetNumFactorOf
  (params (factorOf :type Integer))
  (bind _output_get (LocalVariables|SetrandomNumber (Math|Random|RandomIntegerinRange 1 (- factorOf 1)) :!label _label))
  (while (!= (.Remainder (Math|Float|Division(WholeandRemainder) (Math|Conversions|ToFloat(Integer) factorOf) (Math|Conversions|ToFloat(Integer) _output_get))) 0.0)
    (goto _label))
  (return (LocalVariables|GetrandomNumber)))

(fn GetNumberinRange
  (params (Min :type Integer) (max :type Integer))
  (bind _output_get (LocalVariables|SetrandomNum (Math|Random|RandomIntegerinRange Min max) :!label _label))
  (if (and (<= _output_get max) (>= _output_get Min))
    (return _output_get)
    (else
      (goto _label))))